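; Player character for Le Petit Aventurier, handling Enhanced Input movement, dialogue triggers, item pickup and a slot-based inventory.
; Interaction checks overlapping actors for interfaces, starting dialogues or storing items in the selected empty slot, mirrored in WB_Inventory with mouse-wheel selection.
; Pickups report plane-part counts to the game instance to drive minigame progression.
; The game instance saves player and item data on G; BeginPlay restores transform, inventory and progression.
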(event Custom|Check%20If%20Slot%20empty
  (params (Item%20Details :type BPS%20Items%20Structure) (Current%20Slot :type Integer) (Item%20Ref :type BPA%20Master%20Item%20Object%20Reference))
  (bind _slots_state (Variables|Inventory|GetSlots%20state))
  ;[1 1 1 0.5] Check If Slot is Empty and if Empty = add Item to Slot
  (if (Utilities|Array|Get(acopy) _slots_state Current%20Slot)
    (Development|PrintString "Slot FULL")
    (else
      (bind _item_details (|AddItem&ChangeState Item%20Details Current%20Slot Item%20Ref _slots_state))
      (CallFunction|SetSave&GameProgession _item_details))))

(event Custom|Add%20Item
  (params (Item%20Details :type BPS%20Items%20Structure) (Current%20Slot :type Integer) (Item%20Ref :type BPA%20Master%20Item%20Object%20Reference))
  ;[1 1 1 0.5] Add Item to inventory and set Icon to Widget
  (Utilities|Array|SetArrayElem (Variables|Inventory|GetInventory) Current%20Slot Item%20Details)
  (Default|AddImagetoSlot (Variables|Inventory|GetWB%20Inventory) Current%20Slot (.Icon (Utilities|Struct|BreakBPS_Items Item%20Details)))
  (Actor|DestroyActor Item%20Ref))

(event Custom|Set%20Save%20&%20Game%20Progession
  (params (Item%20Details :type BPS%20Items%20Structure))
  ;[1 1 1 0.5] Set save of Items in Game Instance and change the game progression state
  (bind _result (|CheckIfItemPickedisPlanePart Item%20Details)
    (:%20%20
      (Default|CheckMinigamePlanePartsPicked (Variables|GameInstance|GetGame%20Instance%20Ref) _result))))

(event Input|EnhancedActionEvents|EnhancedInputActionIA_Move
  (params (ActionValue :type Vector%202D%20Structure) (ElapsedSeconds :type Float%20%28double-precision%29) (TriggeredSeconds :type Float%20%28double-precision%29) (InputAction :type Input%20Action%20Object%20Reference :default "/Game/Input/Actions/IA_Move.IA_Move"))
  (bind (_x _y) (Math|Vector2D|BreakVector2D ActionValue))
  ;[1 1 1 0.5] Movement
  ;;[0.005208 0.005208 0.005208 0.5] Right / Left
  (Pawn|Input|AddMovementInput "0.000000,1.000000,0.000000" _x false)
  ;;[0.005208 0.005208 0.005208 0.5] Front / Back
  (Pawn|Input|AddMovementInput "1.000000,0.000000,0.000000" _y false))

(event Input|EnhancedActionEvents|EnhancedInputActionIA_Interaction
  (params (ActionValue :type Boolean) (ElapsedSeconds :type Float%20%28double-precision%29) (TriggeredSeconds :type Float%20%28double-precision%29) (InputAction :type Input%20Action%20Object%20Reference :default "/Game/Le_Petit_Aventurier/Player/Blueprint/Inputs/Actions/IA_Interaction.IA_Interaction"))
  ;[1 1 1 0.5] General Interact
  (:Started
    (for _array_element (Collision|GetOverlappingActors "/Game/Le_Petit_Aventurier/Quests/Plane_Minigame/BPA_Plane_Minigame.BPA_Plane_Minigame_C" :!class /Script/Engine.Actor)
      (if (Utilities|DoesObjectImplementInterface _array_element "/Game/Le_Petit_Aventurier/Interfaces/BPI_Interact.BPI_Interact_C")
        _))))

(event Input|EnhancedActionEvents|EnhancedInputActionIA_Interaction
  (params (ActionValue :type Boolean) (ElapsedSeconds :type Float%20%28double-precision%29) (TriggeredSeconds :type Float%20%28double-precision%29) (InputAction :type Input%20Action%20Object%20Reference :default "/Game/Le_Petit_Aventurier/Player/Blueprint/Inputs/Actions/IA_Interaction.IA_Interaction"))
  ;[1 1 1 0.5] Interaction for Dialogues
  (:Started
    (for _array_element (Collision|GetOverlappingActors "/Game/Le_Petit_Aventurier/Systems/Dialogues/BPA_Dialogue_Character.BPA_Dialogue_Character_C" :!class /Script/Engine.Actor)
      (if (Utilities|DoesObjectImplementInterface _array_element "/Game/Le_Petit_Aventurier/Interfaces/BPI_Dialogue.BPI_Dialogue_C")
        (Default|CallOnCharacterInteraction (Variables|/Game/Le_Petit_Aventurier/Systems/Dialogues/BPA_Dialogue_Character.BPA_Dialogue_Character_C|GetBAC_Dialogues _array_element) (Sprite|GetSprite (Variables|/Game/Le_Petit_Aventurier/Systems/Dialogues/BPA_Dialogue_Character.BPA_Dialogue_Character_C|GetPaperSprite _array_element)))))))

(event Input|EnhancedActionEvents|EnhancedInputActionIA_Interaction
  (params (ActionValue :type Boolean) (ElapsedSeconds :type Float%20%28double-precision%29) (TriggeredSeconds :type Float%20%28double-precision%29) (InputAction :type Input%20Action%20Object%20Reference :default "/Game/Le_Petit_Aventurier/Player/Blueprint/Inputs/Actions/IA_Interaction.IA_Interaction"))
  ;[1 1 1 0.5] Interaction to Pick Up Items
  (:Started
    (for _array_element (Collision|GetOverlappingActors "/Game/Le_Petit_Aventurier/Systems/Inventory/Items/BPA_MasterItem.BPA_MasterItem_C" :!class /Script/Engine.Actor)
      (if (Utilities|DoesObjectImplementInterface _array_element "/Game/Le_Petit_Aventurier/Interfaces/BPI_Interact.BPI_Interact_C")
        (CallFunction|CheckifSlotEmpty (Variables|/Game/Le_Petit_Aventurier/Systems/Inventory/Items/BPA_MasterItem.BPA_MasterItem_C|GetItem%20Details _array_element) (Variables|Inventory|GetCurrent%20Slot) _array_element)))))

(event EventBeginPlay
  ;[1 1 1 0.5] Event Begin Play
  (|AddingMappingInput)
  (|AddWidgetInventory
    (:then2
      (|CreateGameInstance)
      (|GetGameDataandUpdate))))

(event Input|MouseEvents|MouseWheelDown
  (params (Key :type Key%20Structure :default "None"))
  ;[1 1 1 0.5] Navigation between Slots
  (:Pressed
    (if (not (== (Variables|Inventory|GetCurrent%20Slot) (Variables|Inventory|GetMax%20Slots)))
      (bind _result (Math|Integer|IncrementInt (Variables|Inventory|GetCurrent%20Slot))
        (:%20%20
          (Default|ChangeSlots (Variables|Inventory|GetWB%20Inventory) _result))))))

(event Input|MouseEvents|MouseWheelUp
  (params (Key :type Key%20Structure :default "None"))
  ;[1 1 1 0.5] Navigation between Slots
  (:Pressed
    (if (not (== (Variables|Inventory|GetCurrent%20Slot) 0))
      (bind _result (Math|Integer|DecrementInt (Variables|Inventory|GetCurrent%20Slot))
        (:%20%20
          (Default|ChangeSlots (Variables|Inventory|GetWB%20Inventory) _result))))))

(event Input|KeyboardEvents|G
  (params (Key :type Key%20Structure :default "None"))
  (:Pressed
    (bind _player_save (CallFunction|GetPlayerSave))
    (Class|BPISaveGame|SavePlayerData(Message) (Variables|GameInstance|GetGame%20Instance%20Ref) _player_save false)
    (Class|BPISaveGame|SaveItemsData(Message) (Variables|GameInstance|GetGame%20Instance%20Ref) false)
    (Development|PrintString "SAVE DATA")))

(fn ConstructionScript)

(fn GetPlayerSave
  (return (Utilities|Struct|MakeBPS_Player_Save (Transformation|GetActorTransform) (Transformation|GetActorRotation) (Variables|Inventory|GetInventory) (Variables|Inventory|GetSlots%20state) (Variables|Inventory|GetCurrent%20Slot) (Variables|/Game/Le_Petit_Aventurier/Systems/Saves/GI_LePetitAventurier.GI_LePetitAventurier_C|GetGame%20Progression%20State (Variables|GameInstance|GetGame%20Instance%20Ref)))))

(fn UsePlayerSave
  (params (Player%20Save :type BPS%20Player%20Save%20Structure))
  (|PlayerLocation&Rotation (.playerlocation Player%20Save) (.controlrotation Player%20Save))
  (Variables|Inventory|SetInventory (.inventory Player%20Save))
  (Variables|Inventory|SetSlots%20state (.slotemptystate Player%20Save))
  (Variables|Inventory|SetCurrent%20Slot (.currentslot Player%20Save))
  (Variables|/Game/Le_Petit_Aventurier/Systems/Saves/GI_LePetitAventurier.GI_LePetitAventurier_C|SetGame%20Progression%20State (Variables|GameInstance|GetGame%20Instance%20Ref) (.gamestateprogression Player%20Save)))